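; BP_LightFlash is a torch-style spotlight that switches between blue and black when its Toggle event is called.
; Toggle, marked as server, runs only with authority, flipping TorchState and choosing the blue channel value.
; It passes that value to ClientFunction, marked as client, which sets the SpotLight colour.
; The light turns off through black colour rather than a visibility or intensity change.
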(event `Toggle`
  ;[0.1841 0.155 1] Server
  (`/Engine/EditorBlueprintResources/ActorMacros.Switch Has Authority`
    (:`Authority`
      (if (`self.TorchState`)
        (set `self.ColourFloat` 5.0)
        (set `self.TorchState` false)
        (else
          (set `self.ColourFloat` 0.0)
          (set `self.TorchState` true)))
      (`self.ClientFunction` (`self.ColourFloat`)))))

(event `self.ReceiveTick`
  (params (DeltaSeconds :type "Float (single-precision)")))

(event `ClientFunction`
  (params (SetColour :type "Float (double-precision)"))
  ;[0.5103 1 0.9435] Client
  (`LightComponent.SetLightColor` (`self.SpotLight`) (`KismetMathLibrary.MakeColor` 0.0 0.0 SetColour) true))

(fn `UserConstructionScript`)